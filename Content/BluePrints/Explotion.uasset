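; Explosion actor that, on BeginPlay, plays a particle effect, knocks objects back with a radial force impulse and damages nearby actors.
; A sphere trace on the Camera channel, with debug drawing, gathers unique blocking-hit actors that implement DamageInterface.
; Each receives DealDamageMessage with damage falling off linearly by distance within Radius, skipping non-positive values and printing the amount for debugging.
; The actor destroys itself after a short delay.
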(event EventBeginPlay
  (bind _returnvalue (Transformation|GetActorLocation))
  (Components|Activation|Activate (Variables|Default|GetParticleSystem) false)
  ;[1 1 1] knocks back objects with radial force.
  (Variables|/Script/Engine.RadialForceComponent|SetRadius (Variables|Default|GetRadialForce) (Variables|Default|GetRadius))
  (Class|RadialForceComponent|FireImpulse (Variables|Default|GetRadialForce))
  ;[1 1 1] traces a shpere where it hit
  (bind _outhits (Collision|MultiSphereTraceByChannel _returnvalue _returnvalue (Variables|Default|GetRadius) "TraceTypeQuery2" false 0 "ForDuration"))
  (for _array_element _outhits
    ;[1 1 1] saves all hit objects with interface to array
    (if (.bBlockingHit (Collision|BreakHitResult _array_element))
      (if (Utilities|DoesObjectImplementInterface (.HitActor (Collision|BreakHitResult _array_element)) "/Game/BPInterface/DamageInterface.DamageInterface_C")
        (Utilities|Array|AddUnique (Variables|Default|GetDamageableActors) (.HitActor (Collision|BreakHitResult _array_element))))))
  ;[1 1 1] Deals damage to each actor in array
  (for _array_element_2 (Variables|Default|GetDamageableActors)
    (Utilities|IsValid _array_element_2
      (:Is%20Valid
        (Development|PrintString (Utilities|String|ToString(Float) (/ (- (Variables|Default|GetRadius) (Math|Vector|Distance(Vector) (Transformation|GetActorLocation _array_element_2) (Transformation|GetActorLocation))) 1e+01)))
        (if (not (<= (/ (- (Variables|Default|GetRadius) (Math|Vector|Distance(Vector) (Transformation|GetActorLocation _array_element_2) (Transformation|GetActorLocation))) 1e+01) 0.0))
          (Class|DamageInterface|DealDamage(Message) _array_element_2 (/ (- (Variables|Default|GetRadius) (Math|Vector|Distance(Vector) (Transformation|GetActorLocation _array_element_2) (Transformation|GetActorLocation))) 1e+01))))))
  (Utilities|Array|Clear (Variables|Default|GetDamageableActors))
  (Utilities|FlowControl|Delay 0.5)
  (Actor|DestroyActor))

(fn ConstructionScript)