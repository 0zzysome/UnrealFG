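; Game instance Blueprint that tracks enemy waves and holds player and weapon stats for a wave-based combat game.
; Spawn and death events adjust the enemies-left counter, calling HasKilledAllEnemies when it hits zero.
; SpawnWave increments the wave number and calls SpawnNextWave.
; Getter functions return player health and damage resistances, plus fire rates for each weapon type.
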(event EventSpawnWave
  (Math|Integer|IncrementInt (Variables|Default|GetWaveNumber)
    (:%20%20
      (Default|CallSpawnNextWave))))

(event EventEnemyHasDied
  (bind _result (Math|Integer|DecrementInt (Variables|Default|GetEnemiesLeft))
    (:%20%20
      (if (== 0 _result)
        (Default|CallHasKilledAllEnemies)))))

(event EventEnemyHasSpawned
  (Math|Integer|IncrementInt (Variables|Default|GetEnemiesLeft)))

(fn GetPlayerStats
  (return (Variables|PlayerStats|GetCurrentHealth) (Variables|PlayerStats|GetMaxHealth) (Variables|PlayerStats|GetBulletResist) (Variables|PlayerStats|GetExplosiveResist) (Variables|PlayerStats|GetMeleeResist)))

(fn GetPlayerWeaponStats
  (return (Variables|FireRatesWeapons|GetFireRateKnife) (Variables|FireRatesWeapons|GetFireRatePistol) (Variables|FireRatesWeapons|GetFireRateAR) (Variables|FireRatesWeapons|GetFireRateRpg) (Variables|FireRatesWeapons|GetFireRateShotgun) (Variables|FireRatesWeapons|GetFireRateGL)))