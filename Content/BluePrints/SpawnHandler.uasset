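; SpawnHandler spawns waves of AI enemies at placed spawner locations.
; On BeginPlay, if its Spawners array is not empty, it binds SpawnWave to the game instance's SpawnNextWave event.
; Each wave reads enemy counts from the DT_WaveData row named after the current wave number, then spawns both enemy types with their behavior trees, each group at a randomly chosen spawner.
; A missing row only prints "NO MORE WAVES".
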(event Custom|SpawnWave
  (bind _spawners (Variables|Default|GetSpawners))
  (bind _returnvalue (Utilities|Array|Length _spawners))
  (bind _returnvalue_2 (- _returnvalue 1))
  (bind _returnvalue_3 (Math|Random|RandomIntegerinRange 0 _returnvalue_2))
  (bind _output (Utilities|Array|Get(acopy) _spawners _returnvalue_3))
  (bind _returnvalue_4 (Utilities|GetDataTableRow "/Game/BluePrints/DT_WaveData.DT_WaveData" (Utilities|String|StringToName (Utilities|String|ToString(Integer) (Variables|/Game/BluePrints/BPGameInstance.BPGameInstance_C|GetWaveNumber (Variables|Default|GetAs%20BPGame%20Instance)))))
    (:then
      (Utilities|FlowControl|Sequence
        (:then_0
          (CallFunction|SpawnEnemy1 _output (.enemy1 _returnvalue_4)))
        (:then_1
          (CallFunction|SpawnEnemy2 _output (.enemy2 _returnvalue_4)))))
    (:RowNotFound
      (Development|PrintString "NO MORE WAVES"))))

(event EventBeginPlay
  (bind _asbpgame_instance (Utilities|Casting|CastToBPGameInstance (Game|GetGameInstance)))
  (Variables|Default|SetAs%20BPGame%20Instance _asbpgame_instance)
  (if (not (Utilities|Array|IsEmpty (Variables|Default|GetSpawners)))
    (EventDispatchers|BindEventtoSpawnNextWave (Variables|Default|GetAs%20BPGame%20Instance) (delegate Custom|SpawnWave))))

(event Collision|EventActorBeginOverlap
  (params (OtherActor :type Actor%20Object%20Reference)))

(event EventTick
  (params (DeltaSeconds :type Float%20%28single-precision%29)))

(fn ConstructionScript)

(fn SpawnEnemy1
  (params (Location :type Actor%20Object%20Reference) (SpawnAmount :type Integer))
  (for _index (range 0 (- SpawnAmount 1))
    (AI|SpawnAIFromClass "/Game/Enemies/Enemy_test1.Enemy_test1_C" "/Game/Enemies/Enemy1_Tree.Enemy1_Tree" (Transformation|GetActorLocation Location) "0, 0, 0" false 0)))

(fn SpawnEnemy2
  (params (Location :type Actor%20Object%20Reference) (SpawnAmount :type Integer))
  (for _index (range 0 (- SpawnAmount 1))
    (AI|SpawnAIFromClass "/Game/Enemies/Enemy2.Enemy2_C" "/Game/Enemies/Enemy2_Tree.Enemy2_Tree" (Transformation|GetActorLocation Location) "0, 0, 0" false 0)))