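; Firing range spawner actor that spawns target dummies at a set of spawner points.
; On BeginPlay it binds its SpawnDummies event to the game instance's dummy wave spawn event, provided its Spawners list is not empty.
; When SpawnDummies runs, it spawns an Enemy_TargetDummy at the transform of each actor in the list.
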(event Custom|SpawnDummies
  (for _array_element (Variables|Default|GetSpawners)
    (Game|SpawnActorfromClass "/Game/Enemies/TargetDummy/Enemy_TargetDummy.Enemy_TargetDummy_C" (Transformation|GetActorTransform _array_element) "Undefined" "MultiplyWithRoot" 0 0)))

(event EventBeginPlay
  (bind _asbpgame_instance (Utilities|Casting|CastToBPGameInstance (Game|GetGameInstance)))
  (if (not (Utilities|Array|IsEmpty (Variables|Default|GetSpawners)))
    (EventDispatchers|BindEventtoSpawnDummyWave _asbpgame_instance (delegate Custom|SpawnDummies))))

(event Collision|EventActorBeginOverlap
  (params (OtherActor :type Actor%20Object%20Reference)))

(event EventTick
  (params (DeltaSeconds :type Float%20%28single-precision%29)))

(fn ConstructionScript)