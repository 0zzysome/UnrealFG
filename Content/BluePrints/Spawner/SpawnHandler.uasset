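; Spawn manager that creates enemy waves and a pick-one set of random upgrades.
; On the game instance's next-wave event, it reads DT_WaveData by wave number and spawns AI at random spawners, with Shotgun and RPG counts crossed.
; At BeginPlay it spawns one upgrade from a random category at each loot point; destroying any one removes the rest.
; The wave-cleared handler is bound but empty.
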(event Custom|SpawnWave
  (bind _returnvalue (Utilities|GetDataTableRow "/Game/DataTable/DT_WaveData.DT_WaveData" (Utilities|String|StringToName (Utilities|String|ToString(Integer) (Variables|/Game/BluePrints/BPGameInstance.BPGameInstance_C|GetWaveNumber (Variables|Default|GetAs%20BPGame%20Instance)))))
    (:then
      (Utilities|FlowControl|Sequence
        (:then_0
          (EnemySpawns|SpawnEnemyMelee (.enemymele _returnvalue)))
        (:then_1
          (EnemySpawns|SpawnEnemyPistol (.enemypistol _returnvalue)))
        (:then_2
          (EnemySpawns|SpawnEnemyRifle (.enemyrifle _returnvalue)))
        (:then_3
          (EnemySpawns|SpawnEnemyShotgun (.enemyrpg _returnvalue)))
        (:then_4
          (EnemySpawns|SpawnEnemyRPG (.enemyshotgun _returnvalue)))))
    (:RowNotFound
      (Development|PrintString "NO MORE WAVES"))))

(event Custom|OnWaveCleared)

(event Custom|DestroyRest%20of%20options
  (params (DestroyedActor :type Actor%20Object%20Reference))
  (bind _lootlist (Variables|Default|GetLootList))
  (for _array_element _lootlist
    (Utilities|IsValid _array_element
      (:Is%20Valid
        (Actor|DestroyActor _array_element))))
  (Utilities|Array|Clear _lootlist))

(event EventBeginPlay
  (bind _upgrades (Variables|Default|GetUPgrades))
  (bind (_playerupgrades _knifeupgrades _pistolupgrades _rifleupgrades _rocketlauncherupgrades _shotgunupgrades) (Utilities|Struct|BreakS_ClassUpgrade _upgrades))
  (Utilities|FlowControl|Sequence
    (:then_0
      (bind _asbpgame_instance (Utilities|Casting|CastToBPGameInstance (Game|GetGameInstance)))
      (Variables|Default|SetAs%20BPGame%20Instance _asbpgame_instance)
      (if (not (Utilities|Array|IsEmpty (Variables|Default|GetEnemySpawners)))
        (EventDispatchers|BindEventtoSpawnNextWave (Variables|Default|GetAs%20BPGame%20Instance) (delegate Custom|SpawnWave))
        (EventDispatchers|BindEventtoHasCompletedWave (Variables|Default|GetAs%20BPGame%20Instance) (delegate Custom|OnWaveCleared))))
    (:then_1
      (Variables|Upgrades|SetPlayer%20Upgrades _playerupgrades)
      (Variables|Upgrades|SetKnife%20Upgrades _knifeupgrades)
      (Variables|Upgrades|SetPistol%20Upgrades _pistolupgrades)
      (Variables|Upgrades|SetRifle%20Upgrades _rifleupgrades)
      (Variables|Upgrades|SetRocket%20Launcher%20Upgrades _rocketlauncherupgrades)
      (Variables|Upgrades|SetShotgun%20Upgrades _shotgunupgrades))
    (:then_2
      (for _array_element (Variables|Default|GetLootSpawnPoints)
        (CallFunction|SpawnAnyRandomUpgrade (Transformation|GetActorTransform _array_element)))
      (for _array_element_2 (Variables|Default|GetLootList)
        (Game|BindEventtoOnDestroyed _array_element_2 (delegate Custom|DestroyRest%20of%20options))))))

(fn ConstructionScript)

(fn SpawnEnemyMelee
  (params (SpawnAmount :type Integer))
  (bind _enemyspawners (Variables|Default|GetEnemySpawners))
  (for _index (range 0 (- SpawnAmount 1))
    (AI|SpawnAIFromClass "/Game/Enemies/Melee/EnemyMelee.EnemyMelee_C" "/Game/Enemies/Melee/EnemyMelee_Tree.EnemyMelee_Tree" (Transformation|GetActorLocation (Utilities|Array|Get(acopy) _enemyspawners (Math|Random|RandomIntegerinRange 0 (- (Utilities|Array|Length _enemyspawners) 1)))) "0, 0, 0" false 0)))

(fn SpawnEnemyPistol
  (params (SpawnAmount :type Integer))
  (bind _enemyspawners (Variables|Default|GetEnemySpawners))
  (for _index (range 0 (- SpawnAmount 1))
    (AI|SpawnAIFromClass "/Game/Enemies/Pistol/EnemyPistol.EnemyPistol_C" "/Game/Enemies/Pistol/EnemyPistol_Tree.EnemyPistol_Tree" (Transformation|GetActorLocation (Utilities|Array|Get(acopy) _enemyspawners (Math|Random|RandomIntegerinRange 0 (- (Utilities|Array|Length _enemyspawners) 1)))) "0, 0, 0" false 0)))

(fn SpawnEnemyRifle
  (params (SpawnAmount :type Integer))
  (bind _enemyspawners (Variables|Default|GetEnemySpawners))
  (for _index (range 0 (- SpawnAmount 1))
    (AI|SpawnAIFromClass "/Game/Enemies/Rifle/EnemyRifle.EnemyRifle_C" "/Game/Enemies/Rifle/EnemyRifle_Tree.EnemyRifle_Tree" (Transformation|GetActorLocation (Utilities|Array|Get(acopy) _enemyspawners (Math|Random|RandomIntegerinRange 0 (- (Utilities|Array|Length _enemyspawners) 1)))) "0, 0, 0" false 0)))

(fn SpawnEnemyShotgun
  (params (SpawnAmount :type Integer))
  (bind _enemyspawners (Variables|Default|GetEnemySpawners))
  (for _index (range 0 (- SpawnAmount 1))
    (AI|SpawnAIFromClass "/Game/Enemies/ShotGun/ShotgunEnemy.ShotgunEnemy_C" "/Game/Enemies/ShotGun/EnemyShotGun_Tree.EnemyShotGun_Tree" (Transformation|GetActorLocation (Utilities|Array|Get(acopy) _enemyspawners (Math|Random|RandomIntegerinRange 0 (- (Utilities|Array|Length _enemyspawners) 1)))) "0, 0, 0" false 0)))

(fn SpawnEnemyRPG
  (params (SpawnAmount :type Integer))
  (bind _enemyspawners (Variables|Default|GetEnemySpawners))
  (for _index (range 0 (- SpawnAmount 1))
    (AI|SpawnAIFromClass "/Game/Enemies/RPG/EnemyRPG.EnemyRPG_C" "/Game/Enemies/RPG/EnemyRPG_Tree.EnemyRPG_Tree" (Transformation|GetActorLocation (Utilities|Array|Get(acopy) _enemyspawners (Math|Random|RandomIntegerinRange 0 (- (Utilities|Array|Length _enemyspawners) 1)))) "0, 0, 0" false 0)))

(fn SpawnPlayerUpgrade
  (params (SpawnTransform :type Transform))
  (bind _returnvalue (Game|SpawnActorfromClass (.OutItem (Utilities|Array|Random (Variables|Upgrades|GetPlayer%20Upgrades))) SpawnTransform "Undefined" "MultiplyWithRoot" 0 0))
  (Utilities|Array|Add (Variables|Default|GetLootList) _returnvalue))

(fn SpawnKnifeUpgrade
  (params (SpawnTransform :type Transform))
  (bind _returnvalue (Game|SpawnActorfromClass (.OutItem (Utilities|Array|Random (Variables|Upgrades|GetKnife%20Upgrades))) SpawnTransform "Undefined" "MultiplyWithRoot" 0 0))
  (Utilities|Array|Add (Variables|Default|GetLootList) _returnvalue))

(fn SpawnPistolUpgrade
  (params (SpawnTransform :type Transform))
  (bind _returnvalue (Game|SpawnActorfromClass (.OutItem (Utilities|Array|Random (Variables|Upgrades|GetPistol%20Upgrades))) SpawnTransform "Undefined" "MultiplyWithRoot" 0 0))
  (Utilities|Array|Add (Variables|Default|GetLootList) _returnvalue))

(fn SpawnRifleUpgrade
  (params (SpawnTransform :type Transform))
  (bind _returnvalue (Game|SpawnActorfromClass (.OutItem (Utilities|Array|Random (Variables|Upgrades|GetRifle%20Upgrades))) SpawnTransform "Undefined" "MultiplyWithRoot" 0 0))
  (Utilities|Array|Add (Variables|Default|GetLootList) _returnvalue))

(fn SpawnRocketLauncherUpgrade
  (params (SpawnTransform :type Transform))
  (bind _returnvalue (Game|SpawnActorfromClass (.OutItem (Utilities|Array|Random (Variables|Upgrades|GetRocket%20Launcher%20Upgrades))) SpawnTransform "Undefined" "MultiplyWithRoot" 0 0))
  (Utilities|Array|Add (Variables|Default|GetLootList) _returnvalue))

(fn SpawnShotgunUpgrade
  (params (SpawnTransform :type Transform))
  (bind _returnvalue (Game|SpawnActorfromClass (.OutItem (Utilities|Array|Random (Variables|Upgrades|GetShotgun%20Upgrades))) SpawnTransform "Undefined" "MultiplyWithRoot" 0 0))
  (Utilities|Array|Add (Variables|Default|GetLootList) _returnvalue))

(fn SpawnAnyRandomUpgrade
  (params (Spawn%20Transform :type Transform))
  (switch int (Math|Random|RandomIntegerinRange 0 5)
    (:Default
      (Development|PrintString "something whent wrong when spawning"))
    (:0
      (UpgradeSpawns|SpawnPlayerUpgrade Spawn%20Transform))
    (:1
      (UpgradeSpawns|SpawnKnifeUpgrade Spawn%20Transform))
    (:2
      (UpgradeSpawns|SpawnPistolUpgrade Spawn%20Transform))
    (:3
      (UpgradeSpawns|SpawnRifleUpgrade Spawn%20Transform))
    (:4
      (UpgradeSpawns|SpawnRocketLauncherUpgrade Spawn%20Transform))
    (:5
      (UpgradeSpawns|SpawnShotgunUpgrade Spawn%20Transform))))