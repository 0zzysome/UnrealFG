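; Tutorial door actor that opens when the game instance signals that all enemies have been killed.
; On BeginPlay it binds its Opendoor event to the HasKilledAllEnemies dispatcher on BPGameInstance.
; Opendoor plays the Move timeline, rate-scaled by TimeToComplete, to slide the Cube along a Spline, matching its world position and rotation while keeping its scale.
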(event Custom|Opendoor
  (bind _spline (Variables|Default|GetSpline))
  (bind _cube (Variables|Default|GetCube))
  (Components|Timeline|SetPlayRate (Variables|Default|GetMove) (/ 1.0 (Variables|Default|GetTimeToComplete)))
  (bind _move (Timeline|Move Play)
    (:Update
      (Transformation|SetWorldTransform _cube (Math|Transform|MakeTransform (Spline|GetLocationatDistanceAlongSpline _spline (Math|Float|Lerp 0.0 (Spline|GetSplineLength (Variables|Default|GetSpline)) _move) "World") (Spline|GetRotationatDistanceAlongSpline _spline (Math|Float|Lerp 0.0 (Spline|GetSplineLength (Variables|Default|GetSpline)) _move) "World") (Transformation|GetWorldScale _cube)) false false))))

(event Collision|EventActorBeginOverlap
  (params (OtherActor :type Actor%20Object%20Reference)))

(event EventTick
  (params (DeltaSeconds :type Float%20%28single-precision%29)))

(event EventBeginPlay
  (bind _asbpgame_instance (Utilities|Casting|CastToBPGameInstance (Game|GetGameInstance)))
  (EventDispatchers|BindEventtoHasKilledAllEnemies _asbpgame_instance (delegate Custom|Opendoor)))

(fn ConstructionScript)