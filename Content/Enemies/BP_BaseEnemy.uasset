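; Base enemy Blueprint that handles health, resistance-scaled damage and rate-limited shooting, leaving ShootProjectile empty.
; DealDamage applies bullet, explosion and melee damage, fires the health-changed dispatcher, and destroys the actor at zero health.
; Shoot uses a timer with an empty event as a fire-rate cooldown; helper functions check player range and facing.
; It notifies the GameInstance on possession as a spawn and on death.
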(event Custom|CustomEvent)

(event EventPossessed
  (params (NewController :type Controller%20Object%20Reference))
  (Class|SpawnWaveInterface|EnemyHasSpawned(Message) (Game|GetGameInstance)))

(event Collision|EventActorBeginOverlap
  (params (OtherActor :type Actor%20Object%20Reference)))

(event EventDealDamage
  (params (BulletDamage :type Float%20%28double-precision%29) (ExplotionDamage :type Float%20%28double-precision%29) (MeleeDamage :type Float%20%28double-precision%29))
  ;[1 1 1] take damage function.
  (Variables|EnemyStats|SetHealth (Math|Float|Clamp(Float) (- (Variables|EnemyStats|GetHealth) (* BulletDamage (- 1.0 (Variables|EnemyStats|GetBulletResistance)))) 0.0 (Variables|EnemyStats|GetMaxHealth)))
  (Variables|EnemyStats|SetHealth (Math|Float|Clamp(Float) (- (Variables|EnemyStats|GetHealth) (* ExplotionDamage (- 1.0 (Variables|EnemyStats|GetExplotionResistance)))) 0.0 (Variables|EnemyStats|GetMaxHealth)))
  (Variables|EnemyStats|SetHealth (Math|Float|Clamp(Float) (- (Variables|EnemyStats|GetHealth) (* MeleeDamage (- 1.0 (Variables|EnemyStats|GetMeleeResistance)))) 0.0 (Variables|EnemyStats|GetMaxHealth)))
  (Default|CallHealthHasChaged)
  (if (<= (Variables|EnemyStats|GetHealth) 0.0)
    (Class|SpawnWaveInterface|EnemyHasDied(Message) (Game|GetGameInstance))
    (Actor|DestroyActor)))

(event EventShoot
  (if (not (Class|KismetSystemLibrary|TimerExistsHandle (Variables|Default|GetTimerHandle)))
    (CallFunction|ShootProjectile)
    (bind _returnvalue (Utilities|Time|SetTimerbyEvent (delegate Custom|CustomEvent) (Variables|Behavior|GetFireRate)))
    (Variables|Default|SetTimerHandle _returnvalue)))

(fn ConstructionScript)

(fn IsLookingatPlayer
  (return (Utilities|Operators|EqualEqual (Transformation|GetActorRotation) (Math|Rotator|FindLookatRotation (Transformation|GetActorLocation) (Transformation|GetActorLocation (Game|Player|GetPlayerPawn 0))) (Variables|Behavior|GetLookAtPrecision))))

(fn IsPlayerinRange
  (return (< (Math|Vector|Distance(Vector) (Transformation|GetActorLocation) (Transformation|GetActorLocation (Game|Player|GetPlayerPawn 0))) (Variables|Behavior|GetShootRange))))

(fn ShootProjectile)